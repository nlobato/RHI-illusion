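; Trigger volume that runs a keyboard-driven calibration of hand-tracking sensors, showing prompts on a text render while input is enabled on overlap.
; Enter starts calibration, or prompts for recalibration, which R allows.
; Two C presses sample the character's left-hand position for source distance, then center and height, building AxisTranslation with a hard-coded chair height.
; The socket-to-sensor finger-length ratio is only printed for debugging; mesh scaling is disconnected.
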(event OnComponentBeginOverlap(CalibrationVolume)
  (params (OtherActor :type Actor%20Object%20Reference) (OtherComp :type Primitive%20Component%20Object%20Reference) (OtherBodyIndex :type Integer) (bFromSweep :type Boolean) (SweepResult :type Hit%20Result%20Structure%20%28by%20ref%29))
  (bind _textrender (Variables|Default|GetTextRender))
  ;[1 1 1] Text display on Overlap
  (Input|EnableInput (Game|GetPlayerController 0))
  (Rendering|ToggleVisibility _textrender false)
  (Rendering|Components|TextRender|SetText _textrender (Variables|Default|GetInstructions00)))

(event OnComponentEndOverlap(CalibrationVolume)
  (params (OtherActor :type Actor%20Object%20Reference) (OtherComp :type Primitive%20Component%20Object%20Reference) (OtherBodyIndex :type Integer))
  (bind _textrender (Variables|Default|GetTextRender))
  ;[1 1 1] Text display on Overlap
  (Input|DisableInput (Game|GetPlayerController 0))
  (Rendering|ToggleVisibility _textrender false)
  (Rendering|Components|TextRender|SetText _textrender (Variables|Default|GetInstructions00)))

(event Input|KeyboardEvents|Enter
  (params (Key :type Key%20Structure :default "Sensor_13MotionX"))
  (bind _textrender (Variables|Default|GetTextRender))
  ;[1 1 1] Begin Calibration sequence
  (:Pressed
    (if (Variables|Default|GetbIsSystemCalibrated)
      (Rendering|Components|TextRender|SetText _textrender (Variables|Default|GetMessageRecalibration))
      (Variables|Default|SetbIsRecalibrationRequested true)
      (elif (not (Variables|Default|GetbIsCalibrationInProgress))
        (Rendering|Components|TextRender|SetText _textrender (Variables|Default|GetInstructions01))
        (Variables|Default|SetbIsCalibrationInProgress true)))))

(event Input|KeyboardEvents|C
  (params (Key :type Key%20Structure :default "Sensor_13MotionX"))
  (bind _returnvalue (Game|GetPlayerCharacter 0))
  ;[1 1 1] Calibration steps
  (:Pressed
    (if (Variables|Default|GetbIsCalibrationInProgress)
      (if (Variables|Default|GetbIsShoulderHeightCalibrated)
        (bind _asmy_hands_character_bp (Utilities|Casting|CastToMyHands_Character_BP _returnvalue))
        ;;[1 1 1] Obtain center of the person and approximate height
        (Variables|Default|SetSensorValueX (.X (Math|Vector|BreakVector (Class|HandsCharacter|GetLeftHandPosition _asmy_hands_character_bp))))
        (bind _output_get (Variables|Default|SetSensorValueZ (.Z (Math|Vector|BreakVector (Class|HandsCharacter|GetLeftHandPosition _asmy_hands_character_bp)))))
        (Variables|Default|SetAxisTranslation (Math|Vector|MakeVector (Variables|Default|GetSensorValueX) (Variables|Default|GetSensorValueY) (* (- 123.270798 _output_get) -1.0)))
        (Rendering|Components|TextRender|SetText (Variables|Default|GetTextRender) (Variables|Default|GetMessageCalibrationCompleted))
        (Variables|Default|SetbIsSystemCalibrated true)
        (Variables|Default|SetbIsCalibrationInProgress false)
        (Variables|Default|SetbIsShoulderHeightCalibrated false)
        (else
          (bind _asmy_hands_character_bp_2 (Utilities|Casting|CastToMyHands_Character_BP _returnvalue))
          ;;[1 1 1] Obtain distance from source
          (Variables|Default|SetSensorValueY (.Y (Math|Vector|BreakVector (Class|HandsCharacter|GetLeftHandPosition _asmy_hands_character_bp_2))))
          (Development|PrintString (Utilities|String|Append "sockets: " (Utilities|String|ToString(Float) (Math|Vector|VectorLength (- (Transformation|GetSocketLocation (Variables|/Script/Engine.Character|GetMesh _asmy_hands_character_bp_2) "middle_01_lSocket") (Transformation|GetSocketLocation (Variables|/Script/Engine.Character|GetMesh _asmy_hands_character_bp_2) "middle_03_lSocket"))))) true true "(R=1.000000,G=0.043653,B=0.385828,A=1.000000)" 1e+01)
          (Development|PrintString (Utilities|String|Append "sensors: " (Utilities|String|ToString(Float) (Math|Vector|VectorLength (- (Class|HandsCharacter|GetLeftHandPosition _asmy_hands_character_bp_2) (Class|HandsCharacter|GetLeftMiddleFingerPosition _asmy_hands_character_bp_2))))) true true "(R=0.081904,G=1.000000,B=0.127774,A=1.000000)" 1e+01)
          (Development|PrintString (Utilities|String|ToString(Vector) (Math|Conversions|ToVector(Float) (/ (Math|Vector|VectorLength (- (Transformation|GetSocketLocation (Variables|/Script/Engine.Character|GetMesh _asmy_hands_character_bp_2) "middle_01_lSocket") (Transformation|GetSocketLocation (Variables|/Script/Engine.Character|GetMesh _asmy_hands_character_bp_2) "middle_03_lSocket"))) (Math|Vector|VectorLength (- (Class|HandsCharacter|GetLeftHandPosition _asmy_hands_character_bp_2) (Class|HandsCharacter|GetLeftMiddleFingerPosition _asmy_hands_character_bp_2)))))) true true "(R=0.000000,G=0.660000,B=1.000000,A=1.000000)" 1e+01)
          (Rendering|Components|TextRender|SetText (Variables|Default|GetTextRender) (Variables|Default|GetInstructions02))
          (Variables|Default|SetbIsShoulderHeightCalibrated true))))))

(event Input|KeyboardEvents|R
  (params (Key :type Key%20Structure :default "Sensor_13MotionX"))
  ;[1 1 1] Begin Calibration sequence
  (:Pressed
    (if (Variables|Default|GetbIsRecalibrationRequested)
      (Variables|Default|SetbIsSystemCalibrated false))))

(fn ConstructionScript)