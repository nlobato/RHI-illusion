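; InteractionObject_BP is an interactable object whose visible component changes between four preset colors.
; The construction script creates a dynamic material instance from the component's first material and stores it as ObjectColor.
; The ColorChangeEffect event switches on ColorIndex, setting booleans that drive nested SelectColor nodes feeding a vector parameter write.
; That write's parameter name is None, and nothing here changes ColorIndex or calls the event.
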(event EventColorChangeEffect
  (switch int (Variables|Default|GetColorIndex)
    (:0
      (Variables|Default|SetNewVar_0 true)
      (Variables|Default|SetNewVar_1 true)
      (Variables|Default|SetNewVar_2 true))
    (:1
      (Variables|Default|SetNewVar_0 false)
      (Variables|Default|SetNewVar_1 true)
      (Variables|Default|SetNewVar_2 true))
    (:2
      (Variables|Default|SetNewVar_1 false)
      (Variables|Default|SetNewVar_2 true))
    (:3
      (Variables|Default|SetNewVar_2 false)))
  (Rendering|Material|SetVectorParameterValue (Variables|Default|GetObjectColor) "None" (Math|Color|SelectColor (Math|Color|SelectColor (Math|Color|SelectColor "(R=0.006463,G=0.499814,B=0.920000,A=1.000000)" "(R=0.840000,G=0.062177,B=0.000000,A=1.000000)" (Variables|Default|GetNewVar_0)) "(R=0.130296,G=0.700000,B=0.102043,A=1.000000)" (Variables|Default|GetNewVar_1)) "(R=0.905000,G=0.850753,B=0.158375,A=1.000000)" (Variables|Default|GetNewVar_2)) :!class /Script/Engine.MaterialInstanceDynamic))

(event EventBeginPlay)

(event EventActorBeginOverlap
  (params (OtherActor :type Actor%20Object%20Reference)))

(event EventTick
  (params (DeltaSeconds :type Float%20%28single-precision%29)))

(fn ConstructionScript
  (bind _ourvisiblecomponent (Variables|Default|GetOurVisibleComponent))
  (bind _returnvalue (Rendering|Material|CreateDynamicMaterialInstance _ourvisiblecomponent 0 (Utilities|Array|Get(acopy) (Rendering|Material|GetMaterials _ourvisiblecomponent)) :!class /Script/Engine.PrimitiveComponent))
  (Variables|Default|SetObjectColor _returnvalue))