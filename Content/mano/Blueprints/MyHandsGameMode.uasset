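; VR game mode that sets floor-level tracking, spawns a hands character with its body mesh hidden, and places a 3D widget.
; A one-tick delay gates a DoOnce, so alignment and widget placement run only once.
; MoveMesh fits the player character's mesh to the camera by head-socket height and yaw, slightly behind the view.
; Move3DWidget then spawns the widget in front, using that mesh location and rotation.
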(event EventBeginPlay
  (Class|HeadMountedDisplayFunctionLibrary|SetTrackingOrigin "Floor")
  (bind _returnvalue (Game|SpawnActorfromClass "/Game/mano/Blueprints/MyHands_Character_BP.MyHands_Character_BP_C" (Math|Transform|MakeTransform "0.000000,0.000000,10.000000" "0.000000,0.000000,0.000000") "AlwaysSpawn" 0 0))
  (Rendering|SetVisibility (Variables|/Script/Engine.Character|GetMesh _returnvalue) false false))

(event EventTick
  (params (DeltaSeconds :type Float%20%28single-precision%29))
  (if (Variables|Default|GetDoOnce)
    (Utilities|FlowControl|DoOnce false
      (:Completed
        (CallFunction|MoveMesh)
        (CallFunction|Move3DWidget)))
    (else
      (Variables|Default|SetDoOnce true))))

(fn ConstructionScript)

(fn MoveMesh
  (bind _asmy_hands_character_bp (Utilities|Casting|CastToMyHands_Character_BP (Game|GetPlayerCharacter 0)))
  (bind _output_get (Variables|Default|SetMeshLocation (+ (Math|Vector|MakeVector (.X (Math|Vector|BreakVector (.Location (Math|Transform|BreakTransform (Transformation|GetWorldTransform (Variables|/Game/mano/Blueprints/MyHands_Character_BP.MyHands_Character_BP_C|GetCamera _asmy_hands_character_bp)))))) (.Y (Math|Vector|BreakVector (.Location (Math|Transform|BreakTransform (Transformation|GetWorldTransform (Variables|/Game/mano/Blueprints/MyHands_Character_BP.MyHands_Character_BP_C|GetCamera _asmy_hands_character_bp)))))) (- (.Z (Math|Vector|BreakVector (Transformation|GetWorldLocation (Variables|/Script/Engine.Character|GetMesh _asmy_hands_character_bp)))) (- (.Z (Math|Vector|BreakVector (Transformation|GetSocketLocation (Variables|/Script/Engine.Character|GetMesh _asmy_hands_character_bp) "head"))) (/ (.Z (Math|Vector|BreakVector (.Location (Math|Transform|BreakTransform (Transformation|GetWorldTransform (Variables|/Game/mano/Blueprints/MyHands_Character_BP.MyHands_Character_BP_C|GetCamera _asmy_hands_character_bp)))))) 1.0)))) (* (Math|Rotator|GetRotationXVector (Math|Rotator|MakeRotator 0.0 0.0 (.Yaw (Math|Rotator|BreakRotator (.Rotation (Math|Transform|BreakTransform (Transformation|GetWorldTransform (Variables|/Game/mano/Blueprints/MyHands_Character_BP.MyHands_Character_BP_C|GetCamera _asmy_hands_character_bp)))))))) -1e+01))))
  (bind _output_get_2 (Variables|Default|SetMeshRotation (Math|Rotator|CombineRotators (Math|Rotator|MakeRotator 0.0 0.0 (.Yaw (Math|Rotator|BreakRotator (.Rotation (Math|Transform|BreakTransform (Transformation|GetWorldTransform (Variables|/Game/mano/Blueprints/MyHands_Character_BP.MyHands_Character_BP_C|GetCamera _asmy_hands_character_bp))))))) "0,-90.000000, 0")))
  (Transformation|SetWorldLocationAndRotation (Variables|/Script/Engine.Character|GetMesh _asmy_hands_character_bp) _output_get _output_get_2 false false))

(fn Move3DWidget
  (bind _meshrotation (Variables|Default|GetMeshRotation))
  (bind _returnvalue (Math|Rotator|CombineRotators _meshrotation "0,90.000000, 0"))
  (Game|SpawnActorfromClass "/Game/mano/Blueprints/3Dwidget.3Dwidget_C" (Math|Transform|MakeTransform (+ (Variables|Default|GetMeshLocation) (* (Math|Rotator|GetRotationXVector _returnvalue) 4e+02)) _returnvalue) "AlwaysSpawn" 0 0))