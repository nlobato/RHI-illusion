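; CalibrationBox is a trigger volume that walks the player through calibrating hand tracking, with on-screen instructions.
; Overlap toggles the instruction text and enables input only while inside; Enter starts calibration, or clears a completed one.
; C records HandCharacterBP's left-hand Y for the shoulder step, then X and Z on a second press.
; AxisCalibration turns those readings into a translation vector, applying an offset only to Z.
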(event OnComponentBeginOverlap(Box)
  (params (OtherActor :type Actor%20Object%20Reference) (OtherComp :type Primitive%20Component%20Object%20Reference) (OtherBodyIndex :type Integer) (bFromSweep :type Boolean) (SweepResult :type Hit%20Result%20Structure%20%28by%20ref%29))
  (bind _instructionsfirstline (Variables|Default|GetInstructionsFirstLine))
  ;[1 1 1] Text displayed on overlap with collision box
  (Input|EnableInput (Game|GetPlayerController 0))
  (Rendering|ToggleVisibility _instructionsfirstline false)
  (Rendering|Components|TextRender|SetText _instructionsfirstline (Variables|Default|GetInstructions00)))

(event OnComponentEndOverlap(Box)
  (params (OtherActor :type Actor%20Object%20Reference) (OtherComp :type Primitive%20Component%20Object%20Reference) (OtherBodyIndex :type Integer))
  (bind _instructionsfirstline (Variables|Default|GetInstructionsFirstLine))
  ;[1 1 1] Text displayed on overlap with collision box
  (Input|DisableInput (Game|GetPlayerController 0))
  (Rendering|ToggleVisibility _instructionsfirstline false)
  (Rendering|Components|TextRender|SetText _instructionsfirstline (Variables|Default|GetInstructions00)))

(event EventBeginPlay)

(event EventActorBeginOverlap
  (params (OtherActor :type Actor%20Object%20Reference)))

(event EventTick
  (params (DeltaSeconds :type Float%20%28single-precision%29)))

(event Input|KeyboardEvents|Enter
  (params (Key :type Key%20Structure :default "Sensor_7MotionX"))
  (bind _instructionsfirstline (Variables|Default|GetInstructionsFirstLine))
  ;[1 1 1] Calibration initiation
  (:Pressed
    (if (Variables|Default|GetSystemCalibrated)
      (Rendering|Components|TextRender|SetText _instructionsfirstline (Variables|Default|GetMessage))
      (Variables|Default|SetSystemCalibrated false)
      (else
        (Rendering|Components|TextRender|SetText _instructionsfirstline (Variables|Default|GetInstructions01))
        (Variables|Default|SetCalibrationIniated true)))))

(event Input|KeyboardEvents|C
  (params (Key :type Key%20Structure :default "Sensor_7MotionX"))
  (bind _returnvalue (Game|GetPlayerCharacter 0))
  (bind _instructionsfirstline (Variables|Default|GetInstructionsFirstLine))
  ;[1 1 1] Calibration steps
  (:Pressed
    (if (Variables|Default|GetCalibrationIniated)
      (if (Variables|Default|GetShoulderCalibrated)
        (bind _ashand_character_bp (Utilities|Casting|CastToHandCharacterBP _returnvalue))
        (bind _output_get (Variables|Default|SetSensorX (.X (Math|Vector|BreakVector (Variables|/Game/mano/Blueprints/HandCharacterBP.HandCharacterBP_C|GetLeftHandPos _ashand_character_bp)))))
        (bind _output_get_2 (Variables|Default|SetSensorZ (.Z (Math|Vector|BreakVector (Variables|/Game/mano/Blueprints/HandCharacterBP.HandCharacterBP_C|GetLeftHandPos _ashand_character_bp)))))
        (CallFunction|AxisCalibration _output_get (stale _output_get_3) _output_get_2)
        (Rendering|Components|TextRender|SetText _instructionsfirstline (Variables|Default|GetInstructions03))
        (Variables|Default|SetSystemCalibrated true)
        (Variables|Default|SetShoulderCalibrated false)
        (Variables|Default|SetCalibrationIniated false)
        (else
          (bind _ashand_character_bp_2 (Utilities|Casting|CastToHandCharacterBP _returnvalue))
          (bind _output_get_3 (Variables|Default|SetSensorY (.Y (Math|Vector|BreakVector (Variables|/Game/mano/Blueprints/HandCharacterBP.HandCharacterBP_C|GetLeftHandPos _ashand_character_bp_2)))))
          (Rendering|Components|TextRender|SetText _instructionsfirstline (Variables|Default|GetInstructions02))
          (Variables|Default|SetShoulderCalibrated true)))
      (else
        (Rendering|Components|TextRender|SetText (Variables|Default|GetInstructionsFirstLine) (Variables|Default|GetInstructions00))))))

(fn ConstructionScript)

(fn AxisCalibration
  (params (X%20value :type Float%20%28single-precision%29) (Y%20value :type Float%20%28single-precision%29) (Z%20value :type Float%20%28single-precision%29))
  (bind _output_get (Variables|Default|SetAxisTranslation (Math|Vector|MakeVector X%20value Y%20value (* (- (LocalVariables|GetOffsetZ) Z%20value) -1.0))))
  (bind _output_get_2 (Variables|Default|SetAlphaValue 1.0))
  (return _output_get _output_get_2))